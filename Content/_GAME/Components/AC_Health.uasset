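; AC_Health is a health component that tracks an owner's current health, seeded from a starting value plus a stat-based bonus.
; Damage enters through an interface event and passes through server and multicast events to ModifyHealth, so each machine applies it locally.
; ModifyHealth broadcasts the new health and a clamped percentage of starting health, excluding the bonus, then fires OnDeath with the owner when health drops below zero.
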(event Custom|SR_TakeDamage
  (params (Damage :type Float%20%28double-precision%29))
  (CallFunction|MCTakeDamage Damage))

(event Custom|MC_TakeDamage
  (params (Damage :type Float%20%28double-precision%29))
  (CallFunction|ModifyHealth Damage))

(event EventIFTakeDamage
  (params (Damage :type Float%20%28double-precision%29))
  (CallFunction|SRTakeDamage Damage))

(fn Initialize
  (params (Stats :type AC%20Attributes%20Object%20Reference) (Owner :type Actor%20Object%20Reference))
  ;[0.5168 1 0.2131] Set Current Health
  (bind _statvalue (Default|GetStatValue Stats "NewEnumerator0"))
  (Variables|CurrentValues|SetCurrentHealth (+ (* _statvalue 5) (Variables|StartingValues|GetStartingHealth)))
  (Variables|Default|SetOwner Owner))

(fn ModifyHealth
  (params (Damage :type Float%20%28double-precision%29))
  ;[1 1 1] Change Current Health and Send Events accordingly
  (bind _output_get (Variables|CurrentValues|SetCurrentHealth (- (Variables|CurrentValues|GetCurrentHealth) Damage)))
  (Default|CallOnCurrentHealthChanged _output_get)
  (Default|CallOnHealthPercentageChanged (Math|Float|Clamp(Float) (/ (Variables|CurrentValues|GetCurrentHealth) (Variables|StartingValues|GetStartingHealth))))
  ;[1 1 1] Check for Death
  (if (< (Variables|CurrentValues|GetCurrentHealth) 0.0)
    (CallFunction|Die)))

(fn Die
  (Default|CallOnDeath (Variables|Default|GetOwner)))

(fn GetHealth
  (return (Variables|CurrentValues|GetCurrentHealth)))