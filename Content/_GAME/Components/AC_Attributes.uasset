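; Actor component that stores six faith-themed character attributes (Faith, Sanctity, Zeal, Ritualism, Resolve, Purity) and exposes functions to read and change them.
; A helper maps each stat type to a fixed index in the ReplicatedStats integer array.
; ModifyStatValue adds a delta to the stat and clamps the result to that stat's min/max pair in RangesArray.
; BeginPlay and Tick are unused.
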(event EventBeginPlay)

(event EventTick
  (params (DeltaSeconds :type Float%20%28single-precision%29)))

(fn GetStatValue
  (params (StatType :type E_StatType%20Enum :default "NewEnumerator0"))
  (bind _index (CallFunction|PRGetIndexOfStat StatType))
  (return (Utilities|Array|Get(acopy) (Variables|Stats|GetReplicatedStats) _index)))

(fn ModifyStatValue
  (params (StatType :type E_StatType%20Enum :default "NewEnumerator6") (Value :type Integer))
  (LocalVariables|SetL_statType StatType)
  (LocalVariables|SetL_value Value)
  (bind _index (CallFunction|PRGetIndexOfStat (LocalVariables|GetL_statType)))
  (bind _output_get (LocalVariables|SetL_indexOfStat _index))
  (Utilities|Array|SetArrayElem (Variables|Stats|GetReplicatedStats) (LocalVariables|GetL_indexOfStat) (Math|Integer|Clamp(Integer) (+ (LocalVariables|GetL_value) (Utilities|Array|Get(acopy) (Variables|Stats|GetReplicatedStats) _output_get)) (.x (Utilities|Array|Get(acopy) (Variables|Stats|GetRangesArray) (LocalVariables|GetL_indexOfStat))) (.y (Utilities|Array|Get(acopy) (Variables|Stats|GetRangesArray) (LocalVariables|GetL_indexOfStat))))))

(fn PRGetIndexOfStat
  (params (StatType :type E_StatType%20Enum :default "NewEnumerator6"))
  (switch Utilities|FlowControl|Switch|SwitchonE_StatType StatType
    (:NewEnumerator0
      (LocalVariables|SetreturnValue 0))
    (:NewEnumerator1
      (LocalVariables|SetreturnValue 1))
    (:NewEnumerator2
      (LocalVariables|SetreturnValue 2))
    (:NewEnumerator3
      (LocalVariables|SetreturnValue 3))
    (:NewEnumerator4
      (LocalVariables|SetreturnValue 4))
    (:NewEnumerator5
      (LocalVariables|SetreturnValue 5)))
  (return (LocalVariables|GetreturnValue)))