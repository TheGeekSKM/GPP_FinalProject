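; Attribute component for the first-person character that derives health, stamina, sanity and a sprint modifier from Constitution, Dexterity and Intelligence.
; It binds to the owner's sprint and crouch events and adjusts stamina every tick by a drain or regen rate, without delta-time scaling.
; At zero stamina it toggles off sprint and crouch, freezing stamina changes until an exhaustion timer clears.
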(event Custom|OnSprint
  (params (IsSprinting :type Boolean))
  (Variables|States|SetIsSprinting IsSprinting))

(event Custom|ClearExhaustion
  (Variables|States|SetIsExhausted false))

(event Custom|OnCrouch
  (params (IsCrouching :type Boolean))
  (Variables|States|SetIsCrouching IsCrouching))

(event EventBeginPlay
  (Variables|CurrentVariables|SetCurrentHealth (CallFunction|GetMaxHealth))
  (Variables|CurrentVariables|SetCurrentStamina (CallFunction|GetMaxStamina))
  (Variables|CurrentVariables|SetCurrentSanity (CallFunction|GetMaxSanity))
  (bind _asbp_first_person_character (Utilities|Casting|CastToBP_FirstPersonCharacter (Components|GetOwner)))
  (bind _output_get (Variables|Default|SetOwner _asbp_first_person_character))
  (EventDispatchers|BindEventtoOnSprint _output_get (EventDispatchers|CreateEvent :!event Custom|OnSprint))
  (EventDispatchers|BindEventtoOnCrouch _output_get (EventDispatchers|CreateEvent :!event Custom|OnCrouch)))

(event EventTick
  (params (DeltaSeconds :type Float%20%28single-precision%29))
  (CallFunction|HandleStaminaChange))

(fn GetMaxHealth
  (return (* (Variables|Stats|GetConstitution) 1e+01)))

(fn GetSprintModifier
  (return (/ (* (Variables|Stats|GetDexterity) 1e+03) 2e+01)))

(fn GetMaxSanity
  (return (Math|Float|Clamp(Float) (* (- 1e+01 (Variables|Stats|GetIntelligence)) 1e+01) 0.0 1e+02)))

(fn GetMaxStamina
  (return (* (/ (+ (Variables|Stats|GetConstitution) (Variables|Stats|GetDexterity)) 2.0) 1e+02)))

(fn HandleStaminaChange
  (if (not (Variables|States|GetIsExhausted))
    (bind _output_get (Variables|CurrentVariables|SetCurrentStamina (Math|Float|Clamp(Float) (- (Variables|CurrentVariables|GetCurrentStamina) (Math|Float|SelectFloat (Variables|Settings|GetSprintCrouchStaminaDrainRate) (Variables|Settings|GetStaminaRegenRate) (or (Variables|States|GetIsSprinting) (Variables|States|GetIsCrouching)))) 0.0 (CallFunction|GetMaxStamina))))
    (Development|PrintString (Utilities|String|Append "CurrentStamina: " (Utilities|String|ToString(Float) _output_get)))
    (if (<= _output_get 0.0)
      (CallFunction|HandleExhaustion))))

(fn HandleExhaustion
  (Variables|States|SetIsExhausted true)
  (Utilities|Time|SetTimerbyEvent (EventDispatchers|CreateEvent :!event Custom|ClearExhaustion) (Variables|Settings|GetExhaustionTime))
  (Utilities|FlowControl|Sequence
    (:then_0
      (if (Variables|States|GetIsSprinting)
        (Default|ToggleSprint (Variables|Default|GetOwner))))
    (:then_1
      (if (Variables|States|GetIsCrouching)
        (Default|ToggleCrouch (Variables|Default|GetOwner))))))