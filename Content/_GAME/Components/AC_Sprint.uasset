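; Actor component that gives a character toggleable sprinting limited by a stamina pool.
; Initialize sizes max stamina from a base value plus two scaled stats (faith and sanctity) and caches the movement reference.
; Starting or stopping sprint multiplies or divides MaxWalkSpeed and fires OnStaminaChanged with the sprint state.
; Tick drains or regenerates stamina per frame, without delta-time scaling, and stops sprinting when it runs out.
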(event EventTick
  (params (DeltaSeconds :type Float%20%28single-precision%29))
  (if (Variables|Default|GetIsSprinting)
    (bind _result (Math|Float|DecrementFloat (Variables|Default|GetCurrentStamina))
      (:%20%20
        (if (<= _result 0.0)
          (CallFunction|StopSprinting))))
    (elif (< (Variables|Default|GetCurrentStamina) (Variables|Default|GetMaxStamina))
      (Math|Float|IncrementFloat (Variables|Default|GetCurrentStamina)))))

(fn Initialize
  (params (Stats :type AC%20Attributes%20Object%20Reference) (CharacterController :type Character%20Movement%20Component%20Object%20Reference))
  ;[1 1 1] Set Stamina = 100 + ((faith + sanctity) * 4)
  (bind _value (Default|GetStatValue Stats "NewEnumerator1"))
  (bind _value_2 (Default|GetStatValue Stats "NewEnumerator0"))
  (bind _output_get (Variables|Default|SetMaxStamina (+ (* (+ _value_2 _value) 4) (Variables|Default|GetStartingStamina))))
  (Variables|Default|SetCurrentStamina _output_get)
  (Variables|Default|SetCharacter%20Controller CharacterController))

(fn StartSprinting
  (bind _character_controller (Variables|Default|GetCharacter%20Controller))
  (bind _output_get (Variables|/Script/Engine.CharacterMovementComponent|SetMaxWalkSpeed _character_controller (* (Variables|/Script/Engine.CharacterMovementComponent|GetMaxWalkSpeed _character_controller) (Variables|Default|GetAdditionalSpeedMultiplier))))
  (Development|PrintString (Utilities|String|Append "Sprint Speed: " (Utilities|String|ToString(Float) _output_get)))
  (bind _output_get_2 (Variables|Default|SetIsSprinting true))
  (Default|CallOnStaminaChanged _output_get_2))

(fn StopSprinting
  (bind _character_controller (Variables|Default|GetCharacter%20Controller))
  (Variables|/Script/Engine.CharacterMovementComponent|SetMaxWalkSpeed _character_controller (/ (Variables|/Script/Engine.CharacterMovementComponent|GetMaxWalkSpeed _character_controller) (Variables|Default|GetAdditionalSpeedMultiplier)))
  (bind _output_get (Variables|Default|SetIsSprinting false))
  (Default|CallOnStaminaChanged _output_get))

(fn ToggleSprint
  (if (Variables|Default|GetIsSprinting)
    (CallFunction|StopSprinting)
    (else
      (CallFunction|StartSprinting))))