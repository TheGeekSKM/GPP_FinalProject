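; BP_Gun is a gun Blueprint that enables player 0's input and fires a hitscan shot on primary fire.
; Enhanced Input events call start and end functions; primary start checks ammo through the M_CanFire macro, then runs PR_FireBullet.
; The bullet is a debug-drawn Visibility line trace from the camera out to Range, with its hit result unused.
; Secondary fire, primary end and Reload are empty stubs, and ammo is never decremented.
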(event Input|EnhancedActionEvents|EnhancedInputActionIA_ShootPrimary
  (params (ActionValue :type Boolean) (ElapsedSeconds :type Float%20%28double-precision%29) (TriggeredSeconds :type Float%20%28double-precision%29) (InputAction :type Input%20Action%20Object%20Reference :default "/Game/_GAME/FirstPerson/Input/Actions/IA_ShootPrimary.IA_ShootPrimary"))
  (:Started
    (PublicFunctions|StartPrimaryShot))
  (:Canceled
    (PublicFunctions|EndPrimaryShot :!label _label))
  (:Completed
    (goto _label)))

(event Input|EnhancedActionEvents|EnhancedInputActionIA_ShootSecondary
  (params (ActionValue :type Boolean) (ElapsedSeconds :type Float%20%28double-precision%29) (TriggeredSeconds :type Float%20%28double-precision%29) (InputAction :type Input%20Action%20Object%20Reference :default "/Game/_GAME/FirstPerson/Input/Actions/IA_ShootSecondary.IA_ShootSecondary"))
  (:Started
    (PublicFunctions|StartSecondaryShot))
  (:Canceled
    (PublicFunctions|EndSecondaryShot :!label _label))
  (:Completed
    (goto _label)))

(event EventBeginPlay
  (Input|EnableInput (Game|GetPlayerController 0)))

(fn ConstructionScript)

(fn StartPrimaryShot
  (Utilities|MCanFire
    (:HasAmmo
      (PrivateFunctions|PRFireBullet))))

(fn StartSecondaryShot)

(fn Reload)

(fn PRFireBullet
  (bind _returnvalue (Game|GetPlayerCameraManager 0))
  (bind _returnvalue_2 (Transformation|GetActorLocation _returnvalue))
  (Collision|LineTraceByChannel _returnvalue_2 (+ _returnvalue_2 (* (Transformation|GetActorForwardVector _returnvalue) (Variables|Default|GetRange))) "TraceTypeQuery1" false 0 "ForDuration"))

(fn EndPrimaryShot)

(fn EndSecondaryShot)