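; BP_TestObject is a test actor for the game's interaction interface.
; Its IFInteract event prints a debug message saying it has been interacted with, but only when the IsServer flag is true.
; BeginPlay, overlap and Tick are disabled stubs, and the construction script only calls its parent.
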(event EventBeginPlay
  (|CallParentFunction) ; This node is disabled and will not be called.\nDrag off pins to build functionality.
)

(event Collision|EventActorBeginOverlap
  (params (OtherActor :type Actor%20Object%20Reference))
  (|CallParentFunction OtherActor) ; This node is disabled and will not be called.\nDrag off pins to build functionality.
)

(event EventTick
  (params (DeltaSeconds :type Float%20%28single-precision%29))
  (|CallParentFunction DeltaSeconds) ; This node is disabled and will not be called.\nDrag off pins to build functionality.
)

(event EventIFInteract
  (params (Player :type Actor%20Object%20Reference) (IsServer :type Boolean))
  (if IsServer
    (Development|PrintString (Utilities|String|Append "[TestObject] " "I've been interacted with"))))

(fn ConstructionScript
  (|CallParentFunction))