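; BP_WeaponBase is a hitscan weapon, named as a base class, that damages what the camera-aimed trace hits.
; Initialize stores the follow camera and the owner.
; PrimaryFire draws a debug line trace from the camera to its scaled forward vector, which is not offset by the camera's location.
; Hit actors implementing BI_Damageable receive the weapon's damage, with the owner as damage causer.
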(event Collision|EventActorBeginOverlap
  (params (OtherActor :type Actor%20Object%20Reference)))

(event EventTick
  (params (DeltaSeconds :type Float%20%28single-precision%29)))

(fn ConstructionScript)

(fn PrimaryFire
  (bind _follow_camera (Variables|Default|GetFollow%20Camera))
  (bind (_outhit _returnvalue) (Collision|LineTraceByChannel (Transformation|GetWorldLocation _follow_camera) (* (Math|Vector|GetForwardVector _follow_camera) 5e+04) "TraceTypeQuery3" false 0 "ForDuration"))
  (if _returnvalue
    (if (Utilities|DoesObjectImplementInterface (.HitActor (Collision|BreakHitResult _outhit)) "/Game/_GAME/Blueprints/Interfaces/BI_Damageable.BI_Damageable_C")
      (Game|Damage|ApplyDamage (.HitActor (Collision|BreakHitResult _outhit)) (Variables|Default|GetDamage) 0 (Variables|Default|GetWeaponOwner))
      (return))))

(fn Initialize
  (params (FollowCamera :type Camera%20Component%20Object%20Reference) (Owner :type Actor%20Object%20Reference))
  (Variables|Default|SetFollow%20Camera FollowCamera)
  (Variables|Default|SetWeaponOwner Owner))